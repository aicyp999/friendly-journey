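; Softbox light stand Blueprint that provides an adjustable rect light prop for lighting scenes.
; The construction script applies exposed variables for intensity, barn door angle, size, height and tilt.
; It scales, raises and rolls a pivot component, and sizes the rect light source from the same width and height so the two match.
; Its event graph is empty, with no runtime logic.
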(fn `UserConstructionScript`
  (bind _rectlight (`self.RectLight`))
  (bind _rectlight_2 (`self.RectLight`))
  (`LightComponent.SetIntensity` _rectlight (`self.Light Intensity`))
  (`RectLightComponent.SetBarnDoorAngle` _rectlight (`self.Barn Door Angle`))
  (`SceneComponent.SetRelativeScale3D` (`self.ScalePivot`) (`KismetMathLibrary.MakeVector` (`self.Light Width`) 1.0 (`self.Light Height`)))
  (`SceneComponent.K2_SetRelativeLocation` (`self.ScalePivot`) (`KismetMathLibrary.MakeVector` 0.0 44.67 (`self.Height`)) false false)
  (`RectLightComponent.SetSourceWidth` _rectlight_2 (* (`self.Light Width`) 64.0))
  (`RectLightComponent.SetSourceHeight` _rectlight_2 (* (`self.Light Height`) 64.0))
  (`SceneComponent.K2_SetRelativeRotation` (`self.ScalePivot`) (`KismetMathLibrary.MakeRotator` (`self.Light Tilt`)) false false))